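; Player controller for a lap-based racing game that runs the race clock, counts laps and keeps a persistent best time.
; BeginPlay creates the HUD and caches the vehicle pawn, then a one-time Space press starts a Timeline-driven timer that updates the time text.
; UpdateLap increments laps or, once the race is complete, saves any best time and shows the end screen.
; R resets the saved best before the start; P prints debug values.
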(event `self.ReceiveBeginPlay`
  ;[1 1 1] Event Begin Play
  (bind _returnvalue (`|CreateWidget` "/Game/Blueprints/UI/InfoDisplayWidget.InfoDisplayWidget_C"))
  (bind _output_get (set `self.HUDReference` _returnvalue))
  (`UserWidget.AddToViewport` _output_get 0)
  (bind _asvehicle_blueprint (cast `/Game/VehicleAdvBP/Blueprints/VehicleBlueprint` (`GameplayStatics.GetPlayerPawn` 0)))
  (set `self.Vehicle Reference` _asvehicle_blueprint))

(event `StartGameSetUp`
  ;[1 1 1] Start Game Sequence
  (`self.SaveGameCheck`)
  (`self.Init Text`))

(event `StartRaceTime`
  ;[1 1 1] Race Timers
  (bind (_direction _time) (`Timeline|GameTime` :!label _label)
    (:`Update`
      (bind _output_get (set `self.ActualRaceTime` _time))
      (set `self.RaceTimeText` (`/Game/Blueprints/TimeConversion.TimeToText` _output_get)))))

(event `StopRaceTime`
  ;[1 1 1] Race Timers
  (goto _label :!via `Stop`))

(event `UpdateLap`
  ;[1 1 1] Update Lap
  (if (`self.RaceComplete`)
    (`self.RaceTimeCheck`)
    (bind _returnvalue (`|CreateWidget` "/Game/Blueprints/UI/EndWidget.EndWidget_C"))
    (bind _output_get (set `self.NewVar_0` _returnvalue))
    (`UserWidget.AddToViewport` _output_get 0)
    (`self.StopRaceTime`)
    (set `PlayerController.bShowMouseCursor` true (`GameplayStatics.GetPlayerController` 0))
    (else
      (bind _output_get_2 (set `self.ActualLap` (+ (`self.ActualLap`) 1)))
      (set `self.CurrentLapText` (`KismetTextLibrary.Conv_IntToText` _output_get_2)))))

(event `Key|R`
  (params (Key :type "Key Structure"))
  ;[1 1 1] Reset to default
  (:`Pressed`
    (`self.ResetScore`)))

(event `Key|SpaceBar`
  (params (Key :type "Key Structure"))
  (:`Pressed`
    (`/Engine/EditorBlueprintResources/StandardMacros.DoOnce` false
      (:`Completed`
        (`self.PressToStart`)))))

(event `Key|P`
  (params (Key :type "Key Structure"))
  ;[1 1 1] Debug Only
  (:`Pressed`
    (bind _output_get (set `self.BestTimeText` (`KismetTextLibrary.Conv_StringToText` (`KismetStringLibrary.TimeSecondsToString` (`self.BestRaceTime`)))))
    (`KismetSystemLibrary.PrintText` _output_get)
    (bind _output_get_2 (set `self.DefaultBestTimeText` (`KismetTextLibrary.Conv_StringToText` (`KismetStringLibrary.TimeSecondsToString` (`self.DefaultBestRaceTime`)))))
    (`KismetSystemLibrary.PrintText` _output_get_2)
    (bind _output_get_3 (set `self.CurrentLapText` (`KismetTextLibrary.Conv_IntToText` (`self.ActualLap`))))
    (`KismetSystemLibrary.PrintText` _output_get_3)
    (bind _output_get_4 (set `self.MaxLapText` (`KismetTextLibrary.Conv_IntToText` (`self.MaxLaps`))))
    (`KismetSystemLibrary.PrintText` _output_get_4)
    (`KismetSystemLibrary.PrintText` (`KismetTextLibrary.Conv_BoolToText` (`self.RaceComplete`)))))

(fn `Init Text`
  ;[1 1 1] Covert numerical values into text
  (set `self.CurrentLapText` (`KismetTextLibrary.Conv_IntToText` (`self.ActualLap`)))
  (set `self.MaxLapText` (`KismetTextLibrary.Conv_IntToText` (`self.MaxLaps`)))
  (set `self.RaceTimeText` (`/Game/Blueprints/TimeConversion.TimeToText` (`self.ActualRaceTime`)))
  (set `self.BestTimeText` (`/Game/Blueprints/TimeConversion.TimeToText` (`self.BestRaceTime`))))

(fn `LoadTheGame`
  ;[1 1 1] Load game from MySaveGame
  (bind _returnvalue (`GameplayStatics.LoadGameFromSlot` (`self.SaveSlot`)))
  (bind _asmy_save_game (cast `/Game/Blueprints/MySaveGame` _returnvalue))
  (set `self.BestRaceTime` (`/Game/Blueprints/MySaveGame.SavedBestTime` _asmy_save_game)))

(fn `PressToStart`
  (set `/Game/Blueprints/UI/InfoDisplayWidget.GameInfoVisible` "Visible" (`self.HUDReference`))
  (set `self.RaceStart` true)
  (`self.StartRaceTime`))

(fn `RaceTimeCheck`
  ;[1 1 1] Race Time Check
  (if (<= (`self.ActualRaceTime`) (`self.BestRaceTime`))
    (bind _output_get (set `self.BestRaceTime` (`self.ActualRaceTime`)))
    (set `self.BestTimeText` (`/Game/Blueprints/TimeConversion.TimeToText` _output_get))
    (`self.SaveTheGame`)))

(fn `ResetScore`
  (if (not (`self.RaceStart`))
    (set `self.BestRaceTime` (`self.DefaultBestRaceTime`))
    (`self.SaveTheGame`)
    (`self.Init Text`)))

(fn `SaveGameCheck`
  ;[1 1 1] Check Save slots and decide what to do
  (bind _returnvalue (`GameplayStatics.DoesSaveGameExist` (`self.SaveSlot`)))
  (if _returnvalue
    (`self.LoadTheGame`)
    (else
      (set `self.BestRaceTime` (`self.DefaultBestRaceTime`))
      (`self.SaveTheGame`))))

(fn `SaveTheGame`
  ;[1 1 1] Save Game to the Save Slot
  (bind _returnvalue (`GameplayStatics.CreateSaveGameObject` "/Game/Blueprints/MySaveGame.MySaveGame_C"))
  (bind _output_get (set `self.SaveGameReference` _returnvalue))
  (bind _asmy_save_game (cast `/Game/Blueprints/MySaveGame` _output_get))
  (set `/Game/Blueprints/MySaveGame.SavedBestTime` (`self.BestRaceTime`) _asmy_save_game)
  (`GameplayStatics.SaveGameToSlot` (`self.SaveGameReference`) (`self.SaveSlot`)))

(fn `UserConstructionScript`)